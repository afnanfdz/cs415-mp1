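; Actor that spawns and chains BP_Tunnel pieces to build a tunnel.
; On BeginPlay it spawns the first tunnel at the world origin, stores it as NewestTunnel and hands that tunnel a reference back to the spawner.
; SpawnTunnelAtSpawnPoint places the next piece at the world location of the newest tunnel's SpawnPoint, extending the chain whenever it is called.
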(event `self.ReceiveBeginPlay`
  (`self.Spawn Tunnel` (0.0 0.0 0.0)))

(fn `Spawn Tunnel`
  (params (SpawnLocation :type "Vector Structure"))
  (bind _returnvalue (`|SpawnActorFromClass` "/Game/InfiniteMatrix/Blueprints/BP_Tunnel.BP_Tunnel_C" (`KismetMathLibrary.MakeTransform` SpawnLocation) "Undefined" "OverrideRootScale" null null))
  (bind _output_get (set `self.NewestTunnel` _returnvalue))
  (set `/Game/InfiniteMatrix/Blueprints/BP_Tunnel.TunnelSpawner` self _output_get))

(fn `SpawnTunnelAtSpawnPoint`
  (`self.Spawn Tunnel` (`SceneComponent.K2_GetComponentLocation` (`/Game/InfiniteMatrix/Blueprints/BP_Tunnel.SpawnPoint` (`self.NewestTunnel`)))))

(fn `UserConstructionScript`)